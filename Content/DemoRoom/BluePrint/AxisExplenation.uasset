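; AxisExplenation is a demo-room Blueprint that builds a hierarchy of static mesh components mirroring a joint skeleton, apparently to illustrate joint axes.
; The construction script rebuilds the Axies array with one mesh component per joint, 25 in total.
; Each component after the first attaches to its parent joint's component, found by converting the array index to EJoint and calling GetBoneParent.
; The event graph holds no active logic.
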(event EventBeginPlay)

(event EventActorBeginOverlap
  (params (OtherActor :type Actor%20Object%20Reference)))

(event EventTick
  (params (DeltaSeconds :type Float%20%28single-precision%29)))

(fn ConstructionScript
  (Utilities|Array|Clear (Variables|Default|GetAxies))
  (for _index (range 0 24)
    (bind _returnvalue (AddComponent|AddStaticMeshComponent false))
    (Utilities|Array|Add (Variables|Default|GetAxies) _returnvalue))
  (for (_array_element _array_index) (Variables|Default|GetAxies)
    (if (> _array_index 0)
      (Class|SceneComponent|Attachto _array_element (Utilities|Array|Get(acopy) (Variables|Default|GetAxies) (Math|Conversions|ToInteger(Byte) (Class|KinectFunctionLibrary|GetBoneParent (Utilities|Enum|ByteToEnumEJoint (Math|Conversions|ToByte(Integer) _array_index))))) "None" "KeepRelativeOffset" false))))